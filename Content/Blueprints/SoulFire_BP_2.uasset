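; SoulFire pickup actor that adds one to the player's Soulfires count when collected.
; Collection is polled on Tick, requiring player pawn 0 to be within a small horizontal and vertical distance, with no overlap event in use.
; On a successful cast to Player, it increments the count, plays the Take_Coin 2D sound and destroys itself.
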(event `self.ReceiveBeginPlay`)

(event `self.ReceiveTick`
  (params (DeltaSeconds :type "Float (single-precision)"))
  (bind _returnvalue (`GameplayStatics.GetPlayerPawn` 0))
  (if (and (< (`self.GetHorizontalDistanceTo` _returnvalue) 10.0) (< (`self.GetVerticalDistanceTo` _returnvalue) 10.0))
    (bind _asplayer (cast `/Game/Objects/Player` _returnvalue))
    (set `/Game/Objects/Player.Soulfires` (+ (`/Game/Objects/Player.Soulfires` _asplayer) 1) _asplayer)
    (`GameplayStatics.PlaySound2D` "/Game/Media/Take_Coin.Take_Coin")
    (`self.K2_DestroyActor`)))

(fn `UserConstructionScript`)