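; Moving platform actor that shuttles back and forth between its starting position and an EndPoint component.
; On BeginPlay it caches both world locations, sets the timeline play rate from MoveVel and starts the timeline.
; The timeline track drives a lerp of the Platform's location without sweep.
; When it finishes, a location check against either end reverses or replays it, looping the motion.
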(event `self.ReceiveBeginPlay`
  (set `self.Start_Loc` (`SceneComponent.K2_GetComponentLocation` (`self.Platform`)))
  (set `self.End_Loc` (`SceneComponent.K2_GetComponentLocation` (`self.End_Point`)))
  (`TimelineComponent.SetPlayRate` (`self.Platform_Move`) (`self.Move_Vel`))
  (bind (_direction _newtrack_0) (`Timeline|Platform_Move` :!label _label)
    (:`Update`
      (`SceneComponent.K2_SetWorldLocation` (`self.Platform`) (`KismetMathLibrary.VLerp` (`self.Start_Loc`) (`self.End_Loc`) _newtrack_0) false false))
    (:`Finished`
      (if (== (`SceneComponent.K2_GetComponentLocation` (`self.Platform`)) (`self.End_Loc`))
        (goto _label :!via `Reverse`)
        (elif (== (`SceneComponent.K2_GetComponentLocation` (`self.Platform`)) (`self.Start_Loc`))
          (goto _label))))))

(fn `UserConstructionScript`)