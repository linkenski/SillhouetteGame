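; Torch Blueprint that animates a flickering, wandering point light from BeginPlay onward.
; A Flicker timeline drives the light intensity between min and max through its Easing track and requests half-second moves to random relative offsets, scaled by FloatForIncrease.
; When the timeline finishes, it sets the minimum intensity to a fixed value and restarts, so the effect loops indefinitely.
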(event `self.ReceiveBeginPlay`
  (bind (_direction _easing) (`Timeline|Flicker` :!label _label)
    (:`Update`
      (`LightComponent.SetIntensity` (`self.PointLight`) (`KismetMathLibrary.Lerp` (`self.Min_Intensity`) (`self.Max_Intensity`) _easing))
      (`KismetSystemLibrary.MoveComponentTo` (`self.PointLight`) (* (`KismetMathLibrary.RandomUnitVector`) (* (`KismetMathLibrary.RandomFloat`) (`self.Float for increase`))) (struct) false false 0.5))
    (:`Finished`
      (set `self.Min_Intensity` 20000.0)
      (goto _label :!via `PlayFromStart`))))

(fn `UserConstructionScript`)