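; Paper2D slime enemy that patrols between two points and melee-attacks the player when close.
; Construction script feeds PointA and PointB to InterpToMovement; Tick checks health for death, tests player distance and updates animation.
; An attack pauses movement, then after delays enables a collision box that toggles the player's TakesDamage flag on overlap.
; A simple state function picks spawn, idle, run or attack flipbooks, whose lengths time delays.
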(event `Patrol`
  ;[1 1 1] Patrol
  (`ActorComponent.Activate` (`self.InterpToMovement`) false))

(event `Detect Player`
  (bind _returnvalue (`GameplayStatics.GetPlayerPawn` 0))
  (bind _returnvalue_2 (`self.GetHorizontalDistanceTo` _returnvalue))
  (bind _returnvalue_3 (`self.GetVerticalDistanceTo` _returnvalue))
  ;[1 1 1] If Player is near
  (set `self.PlayerTransform` (`self.GetTransform` _returnvalue))
  (set `self.AttackDistance` (`KismetMathLibrary.MakeVector` _returnvalue_2 _returnvalue_3))
  (if (and (< _returnvalue_2 200.0) (<= _returnvalue_3 100.0))
    (`self.Attack Player`)
    (else
      (`self.LeaveHitbox`))))

(event `LeaveHitbox`
  ;[1 1 1] Player leaves hitbox
  (set `self.IsAttacking` false)
  (`PrimitiveComponent.SetCollisionEnabled` (`self.CollisionBox`) "NoCollision")
  (`self.ResetHitbox`)
  (`ActorComponent.SetComponentTickEnabled` (`self.InterpToMovement`) true))

(event `Attack Player`
  ;[1 1 1] Attack Player
  (`/Engine/EditorBlueprintResources/StandardMacros.DoOnce` false :!label _label
    (:`Completed`
      (`ActorComponent.SetComponentTickEnabled` (`self.InterpToMovement`) false)
      (`KismetSystemLibrary.Delay` 0.5)
      (set `self.IsAttacking` true)
      (`KismetSystemLibrary.Delay` 0.5)
      (`PrimitiveComponent.SetCollisionEnabled` (`self.CollisionBox`) "QueryAndPhysics")
      (`KismetSystemLibrary.Delay` (`PaperFlipbookComponent.GetFlipbookLength` (`self.PaperFlipbook`)))
      (`self.LeaveHitbox`))))

(event `self.ReceiveTick`
  (params (DeltaSeconds :type "Float (single-precision)"))
  ;[1 1 1] Update & Routine
  (if (<= (`self.Health`) 0)
    (`self.Die`)
    (else
      (`self.Detect Player`)
      (`self.Update Animation`)
      (`KismetSystemLibrary.Delay` (`PaperFlipbookComponent.GetFlipbookLength` (`self.PaperFlipbook`)))
      (`self.Patrol`))))

(event `ResetHitbox`
  ;[1 1 1] Attack Player
  (goto _label :!via `Reset`))

(event `self.ReceiveBeginPlay`
  ;[1 1 1] Update & Routine
  (`self.EnemyIsSpawning`))

(event `Die`
  (bind _hitbox (`self.Hitbox`))
  ;[1 1 1] Death
  (set `self.Health` 0)
  (`/Engine/EditorBlueprintResources/StandardMacros.DoOnce` false
    (:`Completed`
      (`KismetSystemLibrary.PrintText` "ENEMY DEADED")
      (`/Engine/EditorBlueprintResources/StandardMacros.IsValid` _hitbox
        (:`Is Valid`
          (`self.K2_DestroyActor` _hitbox))
        (:`Is Not Valid`
          _))
      (`self.K2_DestroyActor`))))

(event `EnemyIsSpawning`
  ;[1 1 1] Spawn
  (set `self.IsSpawning` true)
  (`KismetSystemLibrary.Delay` (`PaperFlipbookComponent.GetFlipbookLength` (`self.PaperFlipbook`)))
  (set `self.IsSpawning` false))

(event `self.ReceiveActorBeginOverlap`
  (params (OtherActor :type "Actor Object Reference"))
  ;[1 1 1] Temp Take Damage from player attack
)

(event `Update Animation`
  (bind _x (.x (`self.GetVelocity`)))
  ;[1 1 1] Update Animation
  (set `self.IsIdle` (== _x 0.0))
  (set `self.IsMoving` (!= _x 0.0))
  (set `self.IsAttacking` (`self.IsAttacking`))
  (set `self.IsSpawning` (`self.IsSpawning`))
  (bind _flipbook (`self.AnimationStateMachine` (`self.IsDead`) (`self.IsAttacking`) (`self.IsMoving`) (`self.IsIdle`) (`self.IsSpawning`)))
  (`PaperFlipbookComponent.SetFlipbook` (`self.PaperFlipbook`) _flipbook))

(event `self.CollisionBox.OnComponentBeginOverlap`
  (params (OverlappedComponent :type "PrimitiveComponent Object Reference") (OtherActor :type "Actor Object Reference") (OtherComp :type "PrimitiveComponent Object Reference") (OtherBodyIndex :type Integer) (bFromSweep :type Boolean) (SweepResult :type "HitResult Structure (by ref)"))
  (bind _asplayer (cast `/Game/Objects/Player` OtherActor))
  (if (`ActorComponent.ComponentHasTag` (`Character.CapsuleComponent` _asplayer) "Player")
    (set `/Game/Objects/Player.TakesDamage` true _asplayer)))

(event `self.CollisionBox.OnComponentEndOverlap`
  (params (OverlappedComponent :type "PrimitiveComponent Object Reference") (OtherActor :type "Actor Object Reference") (OtherComp :type "PrimitiveComponent Object Reference") (OtherBodyIndex :type Integer))
  (bind _asplayer (cast `/Game/Objects/Player` OtherActor))
  (if (`ActorComponent.ComponentHasTag` (`Character.CapsuleComponent` _asplayer) "Player")
    (set `/Game/Objects/Player.TakesDamage` false _asplayer)))

(fn `AnimationStateMachine`
  (params (IsDead :type Boolean) (IsAttacking :type Boolean) (IsMoving :type Boolean) (IsIdle :type Boolean) (IsSpawning :type Boolean))
  (returns (Flipbook :type "PaperFlipbook Object Reference"))
  (locals (AnimationState :type "/Game/Objects/AnimationState Enum" :default "NewEnumerator1"))
  (if IsAttacking
    (set `local.AnimationState` "NewEnumerator5")
    (return (select `/Game/Objects/AnimationState` (`local.AnimationState`) :`NewEnumerator0` "/Game/Sprites/Enemy/Slime/Enem_Bl_Slm_Idle.Enem_Bl_Slm_Idle" :`NewEnumerator1` "/Game/Sprites/Enemy/Slime/Enem_Bl_Slm_Idle.Enem_Bl_Slm_Idle" :`NewEnumerator5` "/Game/Sprites/Enemy/Slime/Enem_Bl_Slm_Atk.Enem_Bl_Slm_Atk" :`NewEnumerator8` "/Game/Sprites/Enemy/Slime/Enem_Bl_Slm_Spwn.Enem_Bl_Slm_Spwn" :!type "PaperFlipbook Object Reference"))
    (elif IsMoving
      (set `local.AnimationState` "NewEnumerator0")
      (return (select `/Game/Objects/AnimationState` (`local.AnimationState`) :`NewEnumerator0` "/Game/Sprites/Enemy/Slime/Enem_Bl_Slm_Idle.Enem_Bl_Slm_Idle" :`NewEnumerator1` "/Game/Sprites/Enemy/Slime/Enem_Bl_Slm_Idle.Enem_Bl_Slm_Idle" :`NewEnumerator5` "/Game/Sprites/Enemy/Slime/Enem_Bl_Slm_Atk.Enem_Bl_Slm_Atk" :`NewEnumerator8` "/Game/Sprites/Enemy/Slime/Enem_Bl_Slm_Spwn.Enem_Bl_Slm_Spwn" :!type "PaperFlipbook Object Reference"))
      (elif IsSpawning
        (set `local.AnimationState` "NewEnumerator8")
        (return (select `/Game/Objects/AnimationState` (`local.AnimationState`) :`NewEnumerator0` "/Game/Sprites/Enemy/Slime/Enem_Bl_Slm_Idle.Enem_Bl_Slm_Idle" :`NewEnumerator1` "/Game/Sprites/Enemy/Slime/Enem_Bl_Slm_Idle.Enem_Bl_Slm_Idle" :`NewEnumerator5` "/Game/Sprites/Enemy/Slime/Enem_Bl_Slm_Atk.Enem_Bl_Slm_Atk" :`NewEnumerator8` "/Game/Sprites/Enemy/Slime/Enem_Bl_Slm_Spwn.Enem_Bl_Slm_Spwn" :!type "PaperFlipbook Object Reference"))
        (elif IsIdle
          (set `local.AnimationState` "NewEnumerator1")
          (return (select `/Game/Objects/AnimationState` (`local.AnimationState`) :`NewEnumerator0` "/Game/Sprites/Enemy/Slime/Enem_Bl_Slm_Idle.Enem_Bl_Slm_Idle" :`NewEnumerator1` "/Game/Sprites/Enemy/Slime/Enem_Bl_Slm_Idle.Enem_Bl_Slm_Idle" :`NewEnumerator5` "/Game/Sprites/Enemy/Slime/Enem_Bl_Slm_Atk.Enem_Bl_Slm_Atk" :`NewEnumerator8` "/Game/Sprites/Enemy/Slime/Enem_Bl_Slm_Spwn.Enem_Bl_Slm_Spwn" :!type "PaperFlipbook Object Reference")))))))

(fn `UserConstructionScript`
  (bind _interptomovement (`self.InterpToMovement`))
  (set `InterpToMovementComponent.ControlPoints` (`|MakeArray` (make `InterpControlPoint` (`self.PointA`)) (make `InterpControlPoint` (`self.PointB`))) _interptomovement)
  (`InterpToMovementComponent.FinaliseControlPoints` _interptomovement))