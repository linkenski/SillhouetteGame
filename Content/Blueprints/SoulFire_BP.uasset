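; SoulFire_BP is a fire actor with a flickering point light that casts shadows only when the player is near.
; A looping Flicker timeline lerps light intensity between MinIntensity and MaxIntensity while MoveComponentTo jitters the light toward small random offsets scaled by FloatForIncrease.
; Tick compares the player pawn's distance to the ShadowsOnCollision sphere radius and toggles shadow casting, using a distance check instead of overlap events.
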(event `self.ReceiveTick`
  (params (DeltaSeconds :type "Float (single-precision)"))
  ;[1 1 1] Checks if dynamic shadows should be enabled
  (if (< (`self.GetDistanceTo` (`GameplayStatics.GetPlayerPawn` 0)) (`SphereComponent.SphereRadius` (`self.Shadows_on_collision`)))
    (`LightComponentBase.SetCastShadows` (`self.PointLight`) true)
    (else
      (`LightComponentBase.SetCastShadows` (`self.PointLight`) false))))

(event `self.ReceiveBeginPlay`
  ;[1 1 1] Light flickering
  (bind (_direction _easing) (`Timeline|Flicker` :!label _label)
    (:`Update`
      (`LightComponent.SetIntensity` (`self.PointLight`) (`KismetMathLibrary.Lerp` (`self.Min_Intensity`) (`self.Max_Intensity`) _easing))
      (`KismetSystemLibrary.MoveComponentTo` (`self.PointLight`) (* (* (`KismetMathLibrary.RandomUnitVector`) (* (`KismetMathLibrary.RandomFloat`) (`self.Float for increase`))) 0.5) (struct) false false 0.5))
    (:`Finished`
      (set `self.Min_Intensity` (`self.Min_Intensity`))
      (goto _label :!via `PlayFromStart`))))

(fn `UserConstructionScript`)